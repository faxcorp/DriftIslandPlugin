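; Drift Island plugin actor that builds spline meshes and static-mesh posts along a supplied spline through ConstructFunc.
; It clears old components, then either splits the spline by the scaled first mesh's length, with optional randomization, or copies it.
; CreateSplineMeshes populates each resulting spline.
; The meshes then receive cull distance, collision and translucency sorting, plus optional runtime virtual texture output, sleeping physics and debug count text.
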(fn `Construct Func`
  (params (InputSpline :type "SplineComponent Object Reference") (ParentActor :type "Actor Object Reference") (MeshesForSplines :type "Array of StaticMesh Object Reference") (MeshesForPosts :type "Array of StaticMesh Object Reference") (NumRandomPosts :type Integer) (TangentScale :type "Float (double-precision)") (KnockOutWeight :type "Float (double-precision)") (StraightenPosts :type Boolean) (SetPointsToLinear :type Boolean) (NewSplineForEachSegment :type Boolean) (`SegmentSplineToSplineMeshLength?1` :type Boolean) (Overlap :type "Float (double-precision)") (SegmentScale :type "Float (double-precision)" :default 1.0) (RandomRoll :type "Float (double-precision)") (SplineStart :type "Float (double-precision)") (SplineEnd :type "Float (double-precision)" :default 1.0) (RandomPositionRadius :type "Float (double-precision)") (CullDistanceMin :type Integer) (CullDistanceMax :type Integer) (VirtualTexture :type "RuntimeVirtualTexture Object Reference") (`RenderInMainPass?` :type Boolean) (OffsetSplineTowardsRightVector :type "Float (double-precision)") (OutputStaticMeshesOnSplines :type Boolean) (`EnablePhysicsForStaticMeshes?` :type Boolean) (SplineMeshTranslucencySortPriorityMin :type Integer) (SnapToGround :type Boolean))
  (locals (CurrentSpline :type "SplineComponent Object Reference") (CurrStaticMesh :type "StaticMeshComponent Object Reference"))
  (bind _parentactor (`local.ParentActor`))
  (bind _renderinmainpass_ (`local.RenderInMainPass?`))
  (bind (_returnvalue_origin _returnvalue_boxextent) (`KismetMathLibrary.BreakBoxSphereBounds` (`StaticMesh.GetBounds` (`|GetArrayItem` (`local.MeshesForSplines`)))))
  (`DriftIslandBlueprintFunctionLibrary.DestroyAllComponentsExcept` self (`|MakeArray` (`self.DefaultSceneRoot`)))
  (`/Engine/EditorBlueprintResources/StandardMacros.IsValid` (`local.InputSpline`)
    (:`Is Valid`
      (if (`local.SegmentSplineToSplineMeshLength?1`)
        (bind (_outsplines _returnvalue) (`self.SplitSplineByDistance` (`local.InputSpline`) (* (.x _returnvalue_boxextent) (`local.SegmentScale`) 2.0) (`local.SplineStart`) (`local.SplineEnd`) (`local.SetPointsToLinear`) (`local.NewSplineForEachSegment`) (`local.TangentScale`) (`local.RandomRoll`) (`local.RandomPositionRadius`) self))
        (if (`KismetArrayLibrary.Array_IsValidIndex` _outsplines)
          (for _array_element _outsplines
            (set `local.CurrentSpline` _array_element)
            (`SplineComponent.SetUnselectedSplineSegmentColor` (`local.CurrentSpline`) (make `LinearColor` 1.0 0.0 0.0 1.0) :!label _label)
            (bind (_outstaticmeshesposts _outsplinemeshes) (`self.CreateSplineMeshes` (`local.CurrentSpline`) (select `bool` (`KismetSystemLibrary.IsValid` _parentactor) :`false` self :`true` _parentactor :!type "Actor Object Reference") (`local.MeshesForSplines`) (`local.MeshesForPosts`) (`local.NumRandomPosts`) (`local.CullDistanceMin`) (`local.CullDistanceMax`) (`local.OffsetSplineTowardsRightVector`) 1.0 0.0 (`local.Overlap`) (`local.KnockOutWeight`) (`local.StraightenPosts`) (`local.OutputStaticMeshesOnSplines`) SnapToGround))
            (bind _output_get (set `self.StaticMeshAndSplineMesh` _outstaticmeshesposts))
            (`KismetArrayLibrary.Array_Append` _output_get _outsplinemeshes)
            (set `self.Out Static Meshes Posts` _outstaticmeshesposts)
            (set `self.Out Spline Meshes` _outsplinemeshes)
            (for _array_element_2 (`self.StaticMeshAndSplineMesh`)
              (`/Engine/EditorBlueprintResources/StandardMacros.IsValid` _array_element_2
                (:`Is Valid`
                  (`PrimitiveComponent.SetCullDistance` _array_element_2 (`KismetMathLibrary.Conv_IntToDouble` (/ (+ (`local.CullDistanceMin`) (`local.CullDistanceMax`)) 2)))
                  (`PrimitiveComponent.SetCollisionProfileName` _array_element_2 "BlockAllDynamic" false))))
            (for (_array_element_3 _array_index) (`self.Out Spline Meshes`)
              (`PrimitiveComponent.SetTranslucentSortPriority` _array_element_3 (+ _array_index (`local.SplineMeshTranslucencySortPriorityMin`))))
            (`/Engine/EditorBlueprintResources/StandardMacros.IsValid` (`local.VirtualTexture`)
              (:`Is Valid`
                (for _array_element_4 (`self.Out Spline Meshes`)
                  (`/Engine/EditorBlueprintResources/StandardMacros.IsValid` _array_element_4
                    (:`Is Valid`
                      (set `PrimitiveComponent.RuntimeVirtualTextures` (`|MakeArray` (`local.VirtualTexture`)) _array_element_4)
                      (`PrimitiveComponent.SetRenderInMainPass` _array_element_4 _renderinmainpass_)
                      (if (not _renderinmainpass_)
                        (`PrimitiveComponent.SetCollisionEnabled` _array_element_4 "NoCollision")
                        (`PrimitiveComponent.SetCastShadow` _array_element_4 false))))))
              (:`Is Not Valid`
                _))
            (if (`local.EnablePhysicsForStaticMeshes?`)
              (for _array_element_5 (`self.K2_GetComponentsByClass` "/Script/Engine.StaticMeshComponent")
                (set `local.CurrStaticMesh` _array_element_5)
                (`PrimitiveComponent.SetSimulatePhysics` (`local.CurrStaticMesh`) true)
                (`PrimitiveComponent.SetSimulatePhysics` _array_element_5 true)
                (`PrimitiveComponent.PutRigidBodyToSleep` (`local.CurrStaticMesh`) "None")
                (`PrimitiveComponent.SetMassScale` (`local.CurrStaticMesh`) "None" 10.0)
                (`PrimitiveComponent.SetCollisionObjectType` (`local.CurrStaticMesh`) "ECC_PhysicsBody")
                (`PrimitiveComponent.SetCollisionResponseToChannel` (`local.CurrStaticMesh`) "ECC_PhysicsBody" "ECR_Ignore")))
            (if (`self.DebugText?`)
              (bind _returnvalue_2 (`AddComponent|NODE_AddTextRenderComponent-0`))
              (`TextRenderComponent.K2_SetText` _returnvalue_2 (`KismetTextLibrary.Conv_StringToText` (`KismetStringLibrary.Concat_StrStr` "Num Meshes Posts : " (`KismetStringLibrary.Conv_IntToString` (`KismetArrayLibrary.Array_Length` (`self.Out Static Meshes Posts`))) " --- " "NumSplineMeshes" (`KismetStringLibrary.Conv_IntToString` (`KismetArrayLibrary.Array_Length` (`self.Out Spline Meshes`))) " --- " "NumSplineComponents" (`KismetStringLibrary.Conv_IntToString` (`KismetArrayLibrary.Array_Length` (`self.K2_GetComponentsByClass` "/Script/Engine.SplineComponent"))) " --- " "NumSegmentedSplinePoints" (`KismetStringLibrary.Conv_IntToString` (`SplineComponent.GetNumberOfSplinePoints` (`local.CurrentSpline`))))))))
          (else
            (set `local.CurrentSpline` _returnvalue)
            (goto _label)))
        (else
          (bind _returnvalue_3 (`AddComponent|NODE_AddSplineComponent-0`))
          (bind _output_get_2 (set `local.CurrentSpline` _returnvalue_3))
          (`DriftIslandBlueprintFunctionLibrary.ReplaceSplinePoints` (`local.InputSpline`) _output_get_2 true)
          (goto _label))))))

(fn `UserConstructionScript`)