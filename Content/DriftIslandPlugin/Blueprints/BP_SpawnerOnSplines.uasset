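; Spawner actor that scatters random physics-enabled static meshes alongside name-matched splines, rebuilding them on BeginPlay.
; Regenerate clears generated components, then ConstructFunc orients the splines toward RoadSpline actors and samples seeded random points at a side offset, flipped by the "Reversed" tag.
; Line traces snap points to the ground, and a minimum-spacing check rejects crowded ones until the item or iteration limit.
; Meshes align to spline yaw and start with physics asleep.
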(event `self.ReceiveBeginPlay`
  (`self.Regenerate`))

(event `Regenerate`
  (`self.ClearGeneratedMeshes`)
  (`self.ConstructFunc`))

(event `ClearGeneratedMeshes`
  (`DriftIslandBlueprintFunctionLibrary.DestroyAllComponentsExcept` self (`|MakeArray` (`self.DefaultSceneRoot`))))

(fn `ConstructFunc`
  (locals (FoundActors :type "Array of Actor Object Reference") (CurrSpline :type "SplineComponent Object Reference") (RandomTime :type "Float (double-precision)" :default 0.0))
  (bind (_returnvalue_roll _returnvalue_pitch _returnvalue_yaw) (`KismetMathLibrary.BreakRotator` (`KismetMathLibrary.Conv_VectorToRotator` (* (`SplineComponent.GetDirectionAtTime` (`local.CurrSpline`) (`local.RandomTime`) "World" true) (`KismetMathLibrary.SelectFloat` -1.0 1.0 (`ActorComponent.ComponentHasTag` (`local.CurrSpline`) "Reversed"))))))
  (bind _returnvalue (+ (* (* (`SplineComponent.GetRightVectorAtTime` (`local.CurrSpline`) (`local.RandomTime`) "World" true) (`self.DistanceFromRoad`)) (`KismetMathLibrary.SelectFloat` -1.0 1.0 (`ActorComponent.ComponentHasTag` (`local.CurrSpline`) "Reversed"))) (`SplineComponent.GetLocationAtTime` (`local.CurrSpline`) (`local.RandomTime`) "World" true)))
  (`KismetArrayLibrary.Array_Clear` (`self.Positions`))
  (`KismetMathLibrary.SetRandomStreamSeed` (`self.Random Stream`) (`self.New Seed`))
  (bind _outactors (`GameplayStatics.GetAllActorsOfClass` "/Script/Engine.Actor"))
  (bind _output_get (set `local.FoundActors` (`DriftIslandBlueprintFunctionLibrary.FilterActorsByName` _outactors (`self.Name to Match`))))
  (`DriftIslandBlueprintFunctionLibrary.ReverseSplinesToLookTowardsRoad` _output_get (`DriftIslandBlueprintFunctionLibrary.FilterActorsByName` _outactors "RoadSpline"))
  (set `self.SpawnedItems` 0)
  (for _index (range (+ (`self.MaxTrySpawnIterations`) 1))
    (`KismetMathLibrary.SetRandomStreamSeed` (`self.Random Stream`) (+ (`self.New Seed`) _index))
    (set `local.CurrSpline` (`self.GetComponentByClass` (`KismetArrayLibrary.Array_RandomFromStream` _output_get (`self.Random Stream`)) "/Script/Engine.SplineComponent"))
    (set `local.RandomTime` (`KismetMathLibrary.RandomFloatFromStream` (`self.Random Stream`)))
    (bind _outhit (`KismetSystemLibrary.LineTraceSingle` (+ _returnvalue (0.0 0.0 1000.0)) (+ _returnvalue (0.0 0.0 -1000.0)) "TraceTypeQuery1"))
    (bind (_bblockinghit _binitialoverlap _time _distance _location _impactpoint) (`GameplayStatics.BreakHitResult` _outhit))
    (bind _returnvalue_2 (`KismetMathLibrary.SelectVector` _impactpoint _returnvalue _bblockinghit))
    (bind _returnvalue_3 (`DriftIslandBlueprintFunctionLibrary.IsWithinDistanceOfPositions` (`self.Positions`) (`self.MinimumDistanceBetweenSpawnedItems`) _returnvalue_2))
    (if (not _returnvalue_3)
      (`KismetArrayLibrary.Array_Add` (`self.Positions`) _returnvalue_2)
      (bind _returnvalue_4 (`AddComponent|NODE_AddStaticMeshComponent-0`))
      (`SceneComponent.K2_SetWorldLocationAndRotation` _returnvalue_4 _returnvalue_2 (`KismetMathLibrary.MakeRotator` 0.0 0.0 _returnvalue_yaw) false false)
      (`StaticMeshComponent.SetStaticMesh` _returnvalue_4 (`KismetArrayLibrary.Array_RandomFromStream` (`self.StaticMeshesToSpawn`) (`self.Random Stream`)))
      (`PrimitiveComponent.SetCollisionProfileName` _returnvalue_4 "WorldDynamic" false)
      (`PrimitiveComponent.SetSimulatePhysics` _returnvalue_4 true)
      (`PrimitiveComponent.SetMassScale` _returnvalue_4 "None" 10.0)
      (`PrimitiveComponent.PutRigidBodyToSleep` _returnvalue_4 "None")
      (bind _result (`/Engine/EditorBlueprintResources/StandardMacros.IncrementInt` (`self.SpawnedItems`))
        (:`  `
          (if (>= _result (`self.MaxSpawnedItems`))
            (break)))))))

(fn `UserConstructionScript`)