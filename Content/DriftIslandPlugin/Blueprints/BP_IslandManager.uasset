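; Island manager that clears and rebuilds the island's spline meshes on BeginPlay.
; Each BP_IslandMultiSplineMeshMakerCPP builds from name-matched actors: road makers (Asphalt, Highway, DirtRoad) take all matches, others take seeded random picks without reuse from a shared pool.
; It then sets translucent sort priority on the three intersection instanced meshes so road types layer consistently, and regenerates every BP_SpawnerOnSplines.
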(event `self.ReceiveBeginPlay`
  (`self.ClearAllSplines`)
  (`self.ConstructAllSplines`))

(fn `ClearAllSplines`
  (bind _outactors (`GameplayStatics.GetAllActorsOfClass` "/DriftIslandPlugin/DriftIslandPlugin/Blueprints/BP_IslandMultiSplineMeshMakerCPP.BP_IslandMultiSplineMeshMakerCPP_C"))
  (for _array_element _outactors
    (`/DriftIslandPlugin/DriftIslandPlugin/Blueprints/BP_IslandMultiSplineMeshMakerCPP.ClearSplines` _array_element)))

(fn `ConstructAllSplines`
  (locals (TempArray :type "Array of Actor Object Reference") (NewLocalVar_0 :type Boolean) (OutTemp :type "Actor Object Reference") (CurrSpawner :type "/DriftIslandPlugin/DriftIslandPlugin/Blueprints/BP_IslandMultiSplineMeshMakerCPP Object Reference") (NameMatchString :type String :default "Intersections") (AllActors :type "Array of Actor Object Reference"))
  (bind _temparray (`local.TempArray`))
  (bind _returnvalue (`DriftIslandBlueprintFunctionLibrary.FilterActorsByName` (`self.Splines`) (`local.NameMatchString`)))
  (bind _returnvalue_2 (`DriftIslandBlueprintFunctionLibrary.FilterActorsByName` (`local.AllActors`) (`local.NameMatchString`)))
  (`self.ClearAllSplines`)
  (bind _outactors (`GameplayStatics.GetAllActorsOfClass` "/Script/Engine.Actor"))
  (set `local.AllActors` _outactors)
  (`|ExecutionSequence`
    (:`then_0`
      (`KismetMathLibrary.SetRandomStreamSeed` (`self.Stream`) (`self.New Seed`))
      (set `self.Splines` (`local.AllActors`))
      (bind _outactors_2 (`GameplayStatics.GetAllActorsOfClass` "/DriftIslandPlugin/DriftIslandPlugin/Blueprints/BP_IslandMultiSplineMeshMakerCPP.BP_IslandMultiSplineMeshMakerCPP_C"))
      (for _array_element _outactors_2
        (set `local.CurrSpawner` _array_element)
        (set `local.NameMatchString` (`/DriftIslandPlugin/DriftIslandPlugin/Blueprints/BP_IslandMultiSplineMeshMakerCPP.Name to Match` (`local.CurrSpawner`)))
        (`KismetArrayLibrary.Array_Clear` (`local.TempArray`))
        (if (or (`KismetStringLibrary.Contains` (`local.NameMatchString`) "Asphalt") (`KismetStringLibrary.Contains` (`local.NameMatchString`) "Highway") (`KismetStringLibrary.Contains` (`local.NameMatchString`) "DirtRoad"))
          (if (`KismetArrayLibrary.Array_IsValidIndex` _returnvalue_2)
            (`/DriftIslandPlugin/DriftIslandPlugin/Blueprints/BP_IslandMultiSplineMeshMakerCPP.BuildSplinesFromOtherActor` (`local.CurrSpawner`) _returnvalue_2))
          (else
            (for _index (range (+ (`/DriftIslandPlugin/DriftIslandPlugin/Blueprints/BP_IslandMultiSplineMeshMakerCPP.MaxIterations` (`local.CurrSpawner`)) 1))
              (`KismetMathLibrary.SetRandomStreamSeed` (`self.Stream`) (+ _index (`self.New Seed`)))
              (if (`KismetArrayLibrary.Array_IsValidIndex` (`self.Splines`))
                (if (`KismetArrayLibrary.Array_IsValidIndex` _returnvalue)
                  (set `local.OutTemp` (`KismetArrayLibrary.Array_RandomFromStream` _returnvalue (`self.Stream`)))
                  (`KismetArrayLibrary.Array_Add` (`local.TempArray`) (`local.OutTemp`))
                  (`KismetArrayLibrary.Array_RemoveItem` (`self.Splines`) (`local.OutTemp`)))))
            (if (`KismetArrayLibrary.Array_IsValidIndex` _temparray)
              (`/DriftIslandPlugin/DriftIslandPlugin/Blueprints/BP_IslandMultiSplineMeshMakerCPP.BuildSplinesFromOtherActor` (`local.CurrSpawner`) _temparray))))))
    (:`then_1`
      (`|ExecutionSequence`
        (:`then_0`
          (`PrimitiveComponent.SetTranslucentSortPriority` (`self.GetComponentByClass` (`|GetArrayItem` (`DriftIslandBlueprintFunctionLibrary.FilterActorsByName` (`local.AllActors`) "IntersectionsHighway")) "/Script/Engine.InstancedStaticMeshComponent") 29999))
        (:`then_1`
          (`PrimitiveComponent.SetTranslucentSortPriority` (`self.GetComponentByClass` (`|GetArrayItem` (`DriftIslandBlueprintFunctionLibrary.FilterActorsByName` (`local.AllActors`) "IntersectionsDirtRoad")) "/Script/Engine.InstancedStaticMeshComponent") 9999))
        (:`then_2`
          (`PrimitiveComponent.SetTranslucentSortPriority` (`self.GetComponentByClass` (`|GetArrayItem` (`DriftIslandBlueprintFunctionLibrary.FilterActorsByName` (`local.AllActors`) "IntersectionsAsphalt")) "/Script/Engine.InstancedStaticMeshComponent") 19999))))
    (:`then_2`
      (bind _outactors_3 (`GameplayStatics.GetAllActorsOfClass` "/DriftIslandPlugin/DriftIslandPlugin/Blueprints/BP_SpawnerOnSplines.BP_SpawnerOnSplines_C"))
      (for _array_element_2 _outactors_3
        (`/DriftIslandPlugin/DriftIslandPlugin/Blueprints/BP_SpawnerOnSplines.Regenerate` _array_element_2)))))

(fn `UserConstructionScript`)