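; Island spline mesh builder actor that spawns BP_IslandSplineActor child actors along other actors' splines to lay meshes and posts.
; BuildSplinesEditor defers to BP_IslandManager when one exists; otherwise it clears components and gathers name-matched actors, resized to MaxIterations.
; BuildSplinesFromOtherActor accepts a supplied actor list instead.
; Both paths can reverse splines toward road splines, then attach a child actor per spline, forwarding shared mesh, layout and render settings.
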(event `BuildSplinesEditor`
  (bind _returnvalue (`GameplayStatics.GetActorOfClass` "/DriftIslandPlugin/DriftIslandPlugin/Blueprints/BP_IslandManager.BP_IslandManager_C"))
  (`/Engine/EditorBlueprintResources/StandardMacros.IsValid` _returnvalue
    (:`Is Valid`
      (`/DriftIslandPlugin/DriftIslandPlugin/Blueprints/BP_IslandManager.ConstructAllSplines` _returnvalue))
    (:`Is Not Valid`
      (`DriftIslandBlueprintFunctionLibrary.DestroyAllComponentsExcept` self (`|MakeArray` (`self.DefaultSceneRoot`)))
      (bind _outactors (`GameplayStatics.GetAllActorsOfClass` "/Script/Engine.Actor"))
      (bind _output_get (set `self.ResizedSplineActorArray` (`DriftIslandBlueprintFunctionLibrary.FilterActorsByName` _outactors (`self.Name to Match`))))
      (`KismetArrayLibrary.Array_Resize` _output_get (`self.MaxIterations`))
      (set `self.FoundActors` (`self.ResizedSplineActorArray`))
      (if (or (`self.Reverse All`) (`self.OrientSplinesTowardsOtherSplinesForRoad?`)) :!label _label
        (bind _outactors_2 (`GameplayStatics.GetAllActorsOfClass` "/Script/Engine.Actor"))
        (`DriftIslandBlueprintFunctionLibrary.ReverseSplinesToLookTowardsRoad` (`self.FoundActors`) (`DriftIslandBlueprintFunctionLibrary.FilterActorsByName` _outactors_2 (`self.LookAtSplineNameToMatch`)) (`self.Reverse All`)))
      (for _array_element (`self.FoundActors`)
        (`self.AddSplineMeshMakerComponent` _array_element)))))

(event `BuildSplinesFromOtherActor`
  (params (ActorsWithSplines :type "Array of Actor Object Reference (by ref)"))
  (set `self.FoundActors` ActorsWithSplines)
  (`DriftIslandBlueprintFunctionLibrary.DestroyAllComponentsExcept` self (`|MakeArray` (`self.DefaultSceneRoot`)))
  (goto _label))

(event `self.ReceiveTick`
  (params (DeltaSeconds :type "Float (single-precision)"))
  (`parent.ReceiveTick` DeltaSeconds))

(event `ClearSplines`
  (`DriftIslandBlueprintFunctionLibrary.DestroyAllComponentsExcept` self (`|MakeArray` (`self.DefaultSceneRoot`))))

(fn `AddSplineMeshMakerComponent`
  (params (Spline :type "Actor Object Reference"))
  (bind _returnvalue (`self.GetComponentByClass` Spline "/Script/Engine.SplineComponent"))
  (`/Engine/EditorBlueprintResources/StandardMacros.IsValid` _returnvalue
    (:`Is Valid`
      (bind _returnvalue_2 (`AddComponent|NODE_AddChildActorComponent-0`))
      (`SceneComponent.K2_AttachToComponent` _returnvalue_2 _returnvalue "None" "KeepRelative" "KeepRelative" "KeepRelative" true)
      (bind _asbp_island_spline_actor (cast `/DriftIslandPlugin/DriftIslandPlugin/Blueprints/BP_IslandSplineActor` (`ChildActorComponent.ChildActor` _returnvalue_2)))
      (`/DriftIslandPlugin/DriftIslandPlugin/Blueprints/BP_IslandSplineActor.Construct Func` _asbp_island_spline_actor _returnvalue null (`self.MeshesForSplines`) (`self.MeshesForPosts`) (`self.Num Random Posts`) (`self.Tangent Scale`) (`self.Knock Out Weight`) (`self.Straighten Posts`) (`self.Set Points to Linear`) (`self.New Spline for Each Segment`) (`self.Segment Spline to Spline Mesh Length? 1`) (`self.Overlap`) (`self.Segment Scale`) (`self.Random Roll`) (`self.Spline Start`) (`self.Spline End`) (`self.Random Position Radius`) (`self.Cull Distance Min`) (`self.Cull Distance Max`) (`self.Virtual Texture`) (`self.Render in Main Pass?`) (`self.Offset Spline Towards Right Vector`) (`self.Output Static Meshes on Splines`) (`self.Enable Physics for Static Meshes?`) (`self.Spline Mesh Translucency Sort Priority Min`) (`self.Snap to Ground`)))))

(fn `UserConstructionScript`
  (locals (NewLocalVar_0 :type "Array of SplineComponent Object Reference") (NewLocalVar_1 :type "Array of Actor Object Reference")))